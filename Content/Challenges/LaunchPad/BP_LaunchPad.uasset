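; BP_LaunchPad is a launch pad that throws the player or other components that overlap its Box.
; A BP_Player is launched with a fixed forward-and-up world velocity, independent of pad rotation.
; Anything else gets a velocity-change impulse whose vector is built from the pad's raw rotation angles, not a direction vector.
; An unconnected radial-force loop over overlapping physics components never runs.
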(event `self.ReceiveTick`
  (params (DeltaSeconds :type "Float (single-precision)")))

(event `self.Box.OnComponentBeginOverlap`
  (params (OverlappedComponent :type "PrimitiveComponent Object Reference") (OtherActor :type "Actor Object Reference") (OtherComp :type "PrimitiveComponent Object Reference") (OtherBodyIndex :type Integer) (bFromSweep :type Boolean) (SweepResult :type "HitResult Structure (by ref)"))
  (bind _asbp_player (cast `/Game/Blueprints/BP_Player` OtherActor)
    (:`then`
      (`Character.LaunchCharacter` _asbp_player (1000.0 0.0 1000.0) false false))
    (:`CastFailed`
      (`PrimitiveComponent.AddImpulse` OtherComp (* (`KismetMathLibrary.MakeVector` (+ (.pitch (`self.K2_GetActorRotation`)) 35.0) (.yaw (`self.K2_GetActorRotation`)) (.roll (`self.K2_GetActorRotation`))) 100.0) "None" true))))

(fn `UserConstructionScript`)